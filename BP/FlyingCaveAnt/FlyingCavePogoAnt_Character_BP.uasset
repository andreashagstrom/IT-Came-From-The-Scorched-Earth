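; Flying cave ant creature for ARK that spits projectiles, strips nearby crop plots while untamed, spawns acid on death and hides its rider.
; On server BeginPlay it scales stats from INI multipliers against saved values; CraftMultiplier is applied to speed, not crafting.
; It also destroys itself if the ant count exceeds the INI cap.
; A looping timer runs an octree structure search within an INI-set radius to remove planted crops.
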(event Custom|SearchForCrops
  (bind _self self)
  ;[1 1 1] Destroy Crops
  (if (not (Class|Actor|IsDead _self))
    (if (not (Class|PrimalDinoCharacter|BPIsTamed _self))
      (bind _returnvalue (Class|VictoryCore|ServerOctreeOverlapActors (Class|Actor|GetWorld) (Transformation|GetWorldLocation (Variables|/Script/Engine.Actor|GetStasisCheckComponent self)) (Variables|Default|GetCropSearchRadius) "STRUCTURES" false))
      (for _array_element _returnvalue
        (bind _ascropplotbasebp_c (Utilities|Casting|CastToCropPlotBaseBP _array_element))
        (if (!= (Variables|/Script/ShooterGame.PrimalStructureItemContainer_CropPlot|GetPlantedCrop _ascropplotbasebp_c) 0)
          (Class|PrimalStructureItemContainerCropPlot|RemovePlantedCrop _ascropplotbasebp_c)
          (Development|PrintString "Removed crop.")
          (else
            (Development|PrintString "Found no crop.")))))))

(event Custom|Projectile_MC
  (bind _box1 (Variables|Default|GetBox1))
  (bind _returnvalue (Transformation|GetWorldRotation _box1))
  ;[1 1 1] Spit attack
  (bind _returnvalue_2 (Game|SpawnActorfromClass "/Game/PrimalEarth/CoreBlueprints/Projectiles/ProjArthro.ProjArthro_C" (Math|Transform|MakeTransform (Transformation|GetWorldLocation _box1) _returnvalue) false 0))
  (Class|ShooterProjectile|BPInitVelocity _returnvalue_2 (Math|Vector|GetForwardVector _returnvalue)))

(event EventBeginPlay
  (bind _section (Variables|Default|GetSection))
  (bind _savegametorp (Variables|Default|GetSaveGameTorp))
  (bind _savegamefood (Variables|Default|GetSaveGameFood))
  (bind _savegamestam (Variables|Default|GetSaveGameStam))
  (bind _savegamehealth (Variables|Default|GetSaveGameHealth))
  (|CallParentFunction)
  (Utilities|FlowControl|Delay 0.2)
  (if (Networking|IsServer)
    (bind _asshootergamemode (Utilities|Casting|CastToShooterGameMode (Game|GetGameMode)))
    (Utilities|FlowControl|Sequence
      (:then_0
        ;[1 1 1] Lethals improved statmod
        (bind _returnvalue (Class|PrimalCharacter|GetCharacterStatusComponent))
        (Utilities|FlowControl|Sequence
          (:then_0
            (bind _returnvalue_2 (Class|ShooterGameMode|GetFloatOptionIni _asshootergamemode _section "HealthMultiplier"))
            (Class|PrimalCharacterStatusComponent|SetMaxStatusValue _returnvalue "Health" (* (Math|Float|SelectFloat _returnvalue_2 1.0 (> _returnvalue_2 0.0)) (Class|PrimalCharacterStatusComponent|BPGetMaxStatusValue _returnvalue "Health")))
            (Class|PrimalCharacterStatusComponent|BPDirectSetCurrentStatusValue _returnvalue "Health" (Math|Float|Min(Float) (Class|PrimalCharacterStatusComponent|BPGetMaxStatusValue _returnvalue "Health") (Math|Float|SelectFloat (Math|Float|Max(Float) (Class|PrimalCharacterStatusComponent|BPGetCurrentStatusValue _returnvalue "Health") _savegamehealth) (Class|PrimalCharacterStatusComponent|BPGetMaxStatusValue _returnvalue "Health") (> _savegamehealth 0.0))))
            (Class|PrimalCharacterStatusComponent|UpdatedCurrentStatusValue _returnvalue "Health" (Class|PrimalCharacterStatusComponent|BPGetCurrentStatusValue _returnvalue "Health") true 0 true true))
          (:then_1
            (bind _returnvalue_3 (Class|ShooterGameMode|GetFloatOptionIni _asshootergamemode _section "StamMultiplier"))
            (Class|PrimalCharacterStatusComponent|SetMaxStatusValue _returnvalue "Stamina" (* (Math|Float|SelectFloat _returnvalue_3 1.0 (> _returnvalue_3 0.0)) (Class|PrimalCharacterStatusComponent|BPGetMaxStatusValue _returnvalue "Stamina")))
            (Class|PrimalCharacterStatusComponent|BPDirectSetCurrentStatusValue _returnvalue "Stamina" (Math|Float|Min(Float) (Class|PrimalCharacterStatusComponent|BPGetMaxStatusValue _returnvalue "Stamina") (Math|Float|SelectFloat (Math|Float|Max(Float) (Class|PrimalCharacterStatusComponent|BPGetCurrentStatusValue _returnvalue "Stamina") _savegamestam) (Class|PrimalCharacterStatusComponent|BPGetMaxStatusValue _returnvalue "Stamina") (> _savegamestam 0.0))))
            (Class|PrimalCharacterStatusComponent|UpdatedCurrentStatusValue _returnvalue "Stamina" (Class|PrimalCharacterStatusComponent|BPGetCurrentStatusValue _returnvalue "Stamina") true 0 true true))
          (:then_2
            (bind _returnvalue_4 (Class|ShooterGameMode|GetFloatOptionIni _asshootergamemode _section "WeightMultiplier"))
            (Class|PrimalCharacterStatusComponent|SetMaxStatusValue _returnvalue "Weight" (* (Math|Float|SelectFloat _returnvalue_4 1.0 (> _returnvalue_4 0.0)) (Class|PrimalCharacterStatusComponent|BPGetMaxStatusValue _returnvalue "Weight"))))
          (:then_3
            (bind _returnvalue_5 (Class|ShooterGameMode|GetFloatOptionIni _asshootergamemode _section "DamageMultiplier"))
            (Class|PrimalCharacterStatusComponent|SetMaxStatusValue _returnvalue "MeleeDamageMultiplier" (* (Math|Float|SelectFloat _returnvalue_5 1.0 (> _returnvalue_5 0.0)) (Class|PrimalCharacterStatusComponent|BPGetMaxStatusValue _returnvalue "MeleeDamageMultiplier"))))
          (:then_4
            (bind _returnvalue_6 (Class|ShooterGameMode|GetFloatOptionIni _asshootergamemode _section "SpeedMultiplier"))
            (Class|PrimalCharacterStatusComponent|SetMaxStatusValue _returnvalue "SpeedMultiplier" (* (Math|Float|SelectFloat _returnvalue_6 1.0 (> _returnvalue_6 0.0)) (Class|PrimalCharacterStatusComponent|BPGetMaxStatusValue _returnvalue "SpeedMultiplier"))))
          (:then_5
            (bind _returnvalue_7 (Class|ShooterGameMode|GetFloatOptionIni _asshootergamemode _section "CraftMultiplier"))
            (Class|PrimalCharacterStatusComponent|SetMaxStatusValue _returnvalue "SpeedMultiplier" (* (Math|Float|SelectFloat _returnvalue_7 1.0 (> _returnvalue_7 0.0)) (Class|PrimalCharacterStatusComponent|BPGetMaxStatusValue _returnvalue "SpeedMultiplier"))))
          (:then_6
            (bind _returnvalue_8 (Class|ShooterGameMode|GetFloatOptionIni _asshootergamemode _section "FoodMultiplier"))
            (Class|PrimalCharacterStatusComponent|SetMaxStatusValue _returnvalue "Food" (* (Math|Float|SelectFloat _returnvalue_8 1.0 (> _returnvalue_8 0.0)) (Class|PrimalCharacterStatusComponent|BPGetMaxStatusValue _returnvalue "Food")))
            (Class|PrimalCharacterStatusComponent|BPDirectSetCurrentStatusValue _returnvalue "Food" (Math|Float|Min(Float) (Class|PrimalCharacterStatusComponent|BPGetMaxStatusValue _returnvalue "Food") (Math|Float|SelectFloat (Math|Float|Max(Float) (Class|PrimalCharacterStatusComponent|BPGetCurrentStatusValue _returnvalue "Food") _savegamefood) (Class|PrimalCharacterStatusComponent|BPGetMaxStatusValue _returnvalue "Food") (> _savegamefood 0.0))))
            (Class|PrimalCharacterStatusComponent|UpdatedCurrentStatusValue _returnvalue "Food" (Class|PrimalCharacterStatusComponent|BPGetCurrentStatusValue _returnvalue "Food") true 0 true true))
          (:then_7
            (bind _returnvalue_9 (Class|ShooterGameMode|GetFloatOptionIni _asshootergamemode _section "TorporMultiplier"))
            (Class|PrimalCharacterStatusComponent|SetMaxStatusValue _returnvalue "Torpidity" (* (Math|Float|SelectFloat _returnvalue_9 1.0 (> _returnvalue_9 0.0)) (Class|PrimalCharacterStatusComponent|BPGetMaxStatusValue _returnvalue "Torpidity")))
            (Class|PrimalCharacterStatusComponent|BPDirectSetCurrentStatusValue _returnvalue "Torpidity" (Math|Float|Min(Float) (Class|PrimalCharacterStatusComponent|BPGetMaxStatusValue _returnvalue "Torpidity") (Math|Float|SelectFloat (Math|Float|Min(Float) (Class|PrimalCharacterStatusComponent|BPGetCurrentStatusValue _returnvalue "Torpidity") _savegametorp) (Class|PrimalCharacterStatusComponent|BPGetMaxStatusValue _returnvalue "Torpidity") (> _savegametorp 0.0)) (Class|PrimalCharacterStatusComponent|BPGetCurrentStatusValue _returnvalue "Torpidity")))
            (Class|PrimalCharacterStatusComponent|UpdatedCurrentStatusValue _returnvalue "Torpidity" (Class|PrimalCharacterStatusComponent|BPGetCurrentStatusValue _returnvalue "Torpidity") true 0 true true))
          (:then_8
            (Variables|Default|SetNotSaveGameStatModified true))))
      (:then_1
        ;[1 1 1] Max total ants
        (bind _returnvalue_10 (Class|ShooterGameMode|GetFloatOptionIni _asshootergamemode (Variables|Default|GetSection) "MaxFlyingCaveAnts"))
        (if (<= (Math|Float|Floor _returnvalue_10) 0)
          (Variables|Default|SetMaxAllowed 150)
          (else
            (Variables|Default|SetMaxAllowed (Math|Float|Floor _returnvalue_10))))
        (bind _outactors (Actor|GetAllActorsOfClass "FlyingCavePogoAnt_Character_BP_C"))
        (for (_ _array_index) _outactors
          (if (not (< _array_index (Variables|Default|GetMaxAllowed)))
            (Actor|DestroyActor))))
      (:then_2
        (bind _returnvalue_11 (Class|ShooterGameMode|GetFloatOptionIni _asshootergamemode (Variables|Default|GetSection) "EatCropRadius"))
        (Variables|Default|SetCropSearchRadius (* (Math|Float|SelectFloat _returnvalue_11 6.0 (> _returnvalue_11 0.0)) 3e+02) true)
        (CallFunction|SearchforCrops)
        ;[1 1 1] Destroy Crops
        (Utilities|Time|SetTimerbyEvent (delegate Custom|SearchForCrops) (Variables|Default|GetTimeBetweenCropSearching) true)))))

(event EventOnSetDeath
  (bind _returnvalue (Transformation|GetActorLocation))
  (bind _returnvalue_2 (Math|Conversions|ToTransform(Vector) _returnvalue))
  (bind (_location _rotation) (Math|Transform|BreakTransform _returnvalue_2))
  (Game|SpawnActorfromClass (Variables|Default|GetDeathAcid) (Math|Transform|MakeTransform (+ _location "0, 0,300.000000") _rotation "1.000000,1.000000,1.000000") true))

(fn ConstructionScript
  (|CallParentFunction))

(fn BPNotifySetRider
  (params (RiderSetting :type Shooter%20Character%20Object%20Reference))
  (Rendering|SetActorHiddenInGame RiderSetting true))

(fn BPNotifyClearRider
  (params (RiderClearing :type Shooter%20Character%20Object%20Reference))
  (Rendering|SetActorHiddenInGame RiderClearing false))

(fn DestroyTarget
  (bind _ascropplotbasebp_c (Utilities|Casting|CastToCropPlotBaseBP (Variables|Default|GetTarget)))
  (Class|PrimalStructureItemContainerCropPlot|RemovePlantedCrop _ascropplotbasebp_c))

(fn GetCurrentAttackDuration
  (bind _target (Variables|Default|GetTarget))
  (Utilities|IsValid _target
    (:Is%20Valid
      (Utilities|Casting|CastToPrimalCharacter _target
        (:then
          (LocalVariables|SetAttackDurationValue -1.0))
        (:CastFailed
          (LocalVariables|SetAttackDurationValue (Variables|Default|GetCropAttackDuration))))
      (return (LocalVariables|GetAttackDurationValue)))))

(fn OnRepCropSearchRadius)

(fn BPDoAttack
  (params (AttackIndex :type Integer))
  (if (== AttackIndex 1)
    (CallFunction|ProjectileMC)))